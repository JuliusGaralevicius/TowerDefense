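; Goblin spawner ringed by rocks that spawns goblins on a timer and can be dismantled through interaction.
; The construction script builds a partial ring of rock mesh components from Radius and RockDistance.
; While spawning, it creates goblins above itself, cycling through Paths, until NumberToSpawn is reached.
; Each interaction removes one rock; removing the last notifies TowerDefenseGameMode that the spawner is destroyed.
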(event `self.ReceiveBeginPlay`
  (set `self.TotalPaths` (`KismetArrayLibrary.Array_Length` (`self.Paths`))))

(event `/Game/Interfaces/Interactable.Interact`
  (params (Interactor :type "Actor Object Reference"))
  (`self.RemoveRock`))

(event `RemoveRock`
  (`ActorComponent.K2_DestroyComponent` (`|GetArrayItem` (`self.Rocks`) (`self.CurrentRock`)))
  (bind _result (`/Engine/EditorBlueprintResources/StandardMacros.IncrementInt` (`self.CurrentRock`))
    (:`  `
      (if (>= _result (`KismetArrayLibrary.Array_Length` (`self.Rocks`)))
        (bind _astower_defense_game_mode (cast `/Game/Modes/TowerDefenseGameMode` (`GameplayStatics.GetGameMode`)))
        (`/Game/Modes/TowerDefenseGameMode.OnGoblinSpawnDestroyed` _astower_defense_game_mode self)))))

(event `Start Spawning`
  (`KismetSystemLibrary.K2_SetTimer` null "SpawnActor" (`self.Interval`) true))

(event `Stop Spawning`
  (`KismetSystemLibrary.K2_ClearTimer` null "SpawnActor")
  (set `self.ActorSpawned` 0))

(fn `RequestInteractTIme`
  (returns (success :type Boolean) (Time :type "Float (double-precision)"))
  (return false (`self.RockPickupTime`)))

(fn `SpawnActor`
  (bind _asgoblin_base (castclass `/Game/Characters/Goblins/GoblinBase/GoblinBase` (`self.ActorToSpawn`)))
  (`|SpawnActorFromClass` _asgoblin_base (`KismetMathLibrary.MakeTransform` (+ (`self.K2_GetActorLocation`) (0.0 0.0 100.0))) "AlwaysSpawn" "OverrideRootScale" null (`|GetArrayItem` (`self.Paths`) (`self.NextAvailable`)) null)
  (bind _result (`/Engine/EditorBlueprintResources/StandardMacros.IncrementInt` (`self.ActorSpawned`))
    (:`  `
      (if (>= _result (`self.NumberToSpawn`))
        (`self.Stop Spawning`)
        (return)
        (else
          (bind _result_2 (`/Engine/EditorBlueprintResources/StandardMacros.IncrementInt` (`self.NextAvailable`))
            (:`  `
              (if (== _result_2 (`self.TotalPaths`))
                (set `self.NextAvailable` 0)
                (return)))))))))

(fn `UserConstructionScript`
  (locals (Radius :type "Float (double-precision)" :default 400.0) (SpawnVector :type "Vector Structure" :default (1.0 0.0 0.0)) (RockDistance :type "Float (double-precision)" :default 120.0) (Angle :type "Float (double-precision)") (RockTag :type "Array of Name"))
  (bind _radius (`local.Radius`))
  ;[1 1 1] Spawn rocks around as compinents
  (set `local.SpawnVector` (* (1.0 0.0 0.0) _radius))
  (bind _output_get (set `local.Angle` (/ (`local.RockDistance`) _radius)))
  (bind _returnvalue (- (`KismetMathLibrary.FTrunc` (/ (* (`KismetMathLibrary.GetPI`) 2.0) _output_get)) 2))
  (`KismetArrayLibrary.Array_Resize` (`self.Rocks`) (+ _returnvalue 1))
  (for _index (range (+ _returnvalue 1))
    (bind _returnvalue_2 (`AddComponent|NODE_AddStaticMeshComponent-1` :`RelativeTransform` (`KismetMathLibrary.MakeTransform` (`local.SpawnVector`) (struct) (0.5 0.5 0.5))))
    (`StaticMeshComponent.SetStaticMesh` _returnvalue_2 "/Game/Environment/LowPolyFoliage/Rocks/Rock_11.Rock_11")
    (`PrimitiveComponent.SetCollisionResponseToChannel` _returnvalue_2 "ECC_GameTraceChannel1" "ECR_Block")
    (`KismetArrayLibrary.Array_Set` (`self.Rocks`) _index _returnvalue_2 true)
    (set `local.SpawnVector` (`KismetMathLibrary.RotateAngleAxis` (`local.SpawnVector`) (`KismetMathLibrary.RadiansToDegrees` (`local.Angle`)) (0.0 0.0 1.0)))))