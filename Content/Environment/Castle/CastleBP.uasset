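; Player castle for the tower defense mode, with destructible walls whose total collapse ends the game.
; BeginPlay maps each tagged wall's collider to its tiers and health bar, and builds melee and ranged rings of attack slots.
; DamageDealer overlaps reduce wall health, swapping top, middle and bottom meshes for hidden destructibles at each third lost.
; Helpers supply the nearest wall or free ranged slot, while manually redrawn health bars face the camera.
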(event `self.ReceiveTick`
  (params (DeltaSeconds :type "Float (single-precision)"))
  (`self.WidgetsFaceCamera`))

(event `self.ReceiveBeginPlay`
  (bind _locs (`self.CreateSpawns` 200.0 (`SphereComponent.GetScaledSphereRadius` (`self.StackingRadius`))))
  (set `self.MeleeLocations` _locs)
  (bind _locs_2 (`self.CreateSpawns` 200.0 (`SphereComponent.GetScaledSphereRadius` (`self.RangeRadius`))))
  (set `self.RangedLocations` _locs_2)
  (bind _output_get (set `self.WallRoots` (`self.GetComponentsByTag` self "/Script/Engine.SceneComponent" "wall")))
  (`self.PopulateMap` _output_get (`self.HealthPerWall`))
  (bind _keys (`BlueprintMapLibrary.Map_Keys` (`self.ColliderToStruct`)))
  (for _array_element _keys
    (add `PrimitiveComponent.OnComponentBeginOverlap` _array_element (delegate `CustomEvent_0`)))
  (`self.SetupVisibility`)
  (`KismetSystemLibrary.Delay` 0.2)
  (bind _astower_defense_game_mode (cast `/Game/Modes/TowerDefenseGameMode` (`GameplayStatics.GetGameMode`)))
  (set `/Game/Modes/TowerDefenseGameMode.PlayerCastle` self _astower_defense_game_mode))

(event `CustomEvent_0`
  (params (OverlappedComponent :type "PrimitiveComponent Object Reference") (OtherActor :type "Actor Object Reference") (OtherComp :type "PrimitiveComponent Object Reference") (OtherBodyIndex :type Integer) (bFromSweep :type Boolean) (SweepResult :type "HitResult Structure (by ref)"))
  (bind _asbox_collision (cast `BoxComponent` OverlappedComponent))
  (bind _asdamage_dealer (cast `/Game/Interfaces/DamageDealer` OtherActor))
  (bind _damage (`/Game/Interfaces/DamageDealer.OnRequestDamage` _asdamage_dealer))
  (`self.DamageWall` self _asbox_collision _damage)
  (`KismetSystemLibrary.PrintString` (`KismetStringLibrary.Conv_DoubleToString` _damage)))

(fn `CollapseWall`
  (params (wall :type "StaticMeshComponent Object Reference (by ref)") (wallDestructible :type "DestructibleComponent Object Reference (by ref)") (ImpactPoint :type "Vector Structure (by ref)"))
  (bind _wall (`local.wall`))
  (bind _walldestructible (`local.wallDestructible`))
  (if (not (`SceneComponent.bVisible` wallDestructible))
    (`SceneComponent.SetVisibility` _wall false false)
    (`PrimitiveComponent.SetCollisionEnabled` _wall "NoCollision")
    (`SceneComponent.SetVisibility` _walldestructible true false)
    (`PrimitiveComponent.SetCollisionEnabled` _walldestructible "QueryAndPhysics")
    (`DestructibleComponent.ApplyRadiusDamage` _walldestructible 100.0 (`local.ImpactPoint`) 2000.0 100.0 true)
    (return)))

(fn `CreateSpawns`
  (params (Gap :type "Float (double-precision)" :default 100.0) (Radius :type "Float (double-precision)"))
  (returns (Locs :type "Array of /Game/Environment/Castle/AttackLocation Structure"))
  (locals (Locations :type "Array of Vector Structure") (SpawnLocation :type "Vector Structure") (Angle :type "Float (double-precision)") (LocationArray :type "Array of /Game/Environment/Castle/AttackLocation Structure"))
  (bind _locationarray (`local.LocationArray`))
  (bind _radius (`local.Radius`))
  (bind _astower_defense_game_mode (cast `/Game/Modes/TowerDefenseGameMode` (`GameplayStatics.GetGameMode`)))
  (set `/Game/Modes/TowerDefenseGameMode.PlayerCastle` self _astower_defense_game_mode)
  (set `local.SpawnLocation` (* (1.0 0.0 0.0) _radius))
  (bind _output_get (set `local.Angle` (/ (`local.Gap`) _radius)))
  (bind _returnvalue (`KismetMathLibrary.FTrunc` (/ (* (`KismetMathLibrary.GetPI`) 2.0) _output_get)))
  (`KismetArrayLibrary.Array_Resize` _locationarray (+ _returnvalue 1))
  (for _index (range (+ _returnvalue 1))
    (`KismetArrayLibrary.Array_Set` _locationarray _index (make `/Game/Environment/Castle/AttackLocation` true (+ (`local.SpawnLocation`) (0.0 0.0 50.0) (`self.K2_GetActorLocation` self))) true)
    (set `local.SpawnLocation` (`KismetMathLibrary.RotateAngleAxis` (`local.SpawnLocation`) (`KismetMathLibrary.RadiansToDegrees` (`local.Angle`)) (0.0 0.0 1.0))))
  (return (`local.LocationArray`)))

(fn `DamageWall`
  (params (WallCollider :type "BoxComponent Object Reference") (Damage :type "Float (double-precision)" :default 50.0))
  (locals (WallStruct :type "/Game/Environment/Castle/Wall Structure") (Health :type "Float (double-precision)"))
  (bind (_wallstruct_destructibletop _wallstruct_destructiblemiddle _wallstruct_destructiblebottom _wallstruct_topwall _wallstruct_midwall _wallstruct_botwall) (break `/Game/Environment/Castle/Wall` (`local.WallStruct`)))
  (bind _wallstruct (`local.WallStruct`))
  (bind _healthperwall (`self.HealthPerWall`))
  (bind (_destructibletop _destructiblemiddle _destructiblebottom _topwall _midwall _botwall _health _healthbarcomponent _healthbarwidget) (break `/Game/Environment/Castle/Wall` _wallstruct))
  (bind (_value _returnvalue) (`BlueprintMapLibrary.Map_Find` (`self.ColliderToStruct`) WallCollider))
  (bind _returnvalue_2 (`SceneComponent.K2_GetComponentLocation` (`local.WallCollider`)))
  (if _returnvalue
    (bind _output_get (set `local.WallStruct` _value))
    (bind _returnvalue_3 (- (`.Health_17_0327A4744A1727857AB9DFB28249C054` (break `/Game/Environment/Castle/Wall` _output_get)) (`local.Damage`)))
    (setmembers `/Game/Environment/Castle/Wall` :`StructRef` (`local.WallStruct`) :`Health` _returnvalue_3)
    (`self.checkRange` (* _healthperwall 0.0) (* _healthperwall 0.33) (* _healthperwall 0.66) _returnvalue_3
      (:`less than 1`
        (`self.CollapseWall` _wallstruct_botwall _wallstruct_destructiblebottom _returnvalue_2)
        (bind _astower_defense_game_mode (cast `/Game/Modes/TowerDefenseGameMode` (`GameplayStatics.GetGameMode`)))
        (`/Game/Modes/TowerDefenseGameMode.EndGame` _astower_defense_game_mode)
        (`KismetSystemLibrary.PrintString` "Hello"))
      (:`1 to 2`
        (`self.CollapseWall` _wallstruct_midwall _wallstruct_destructiblemiddle _returnvalue_2)
        (`BlueprintMapLibrary.Map_Add` (`self.ColliderToStruct`) (`local.WallCollider`) _wallstruct :!label _label)
        (`KismetSystemLibrary.PrintString` (`KismetStringLibrary.Conv_DoubleToString` _returnvalue_3))
        (`/Game/UI/HealthBar.Health Change` _healthbarwidget (/ _health (`self.HealthPerWall`)))
        (`WidgetComponent.RequestRedraw` _healthbarcomponent)
        (return))
      (:`2 to 3`
        (`self.CollapseWall` _wallstruct_topwall _wallstruct_destructibletop _returnvalue_2)
        (goto _label))
      (:`3 or more`
        (goto _label)))))

(fn `GetClosestLocation`
  (params (searchLocation :type "Vector Structure") (Ranged :type Boolean :default true))
  (returns (AttackLocation :type "Vector Structure") (Index :type Integer))
  (locals (CurrentMin :type "Float (double-precision)" :default 1000000000.0) (CurrentBestVector :type "Vector Structure") (CurrentBestIndex :type Integer))
  (if Ranged
    (for (_array_element _array_index) (`self.RangedLocations`)
      (if (break `/Game/Environment/Castle/AttackLocation` _array_element)
        (bind _returnvalue (`KismetMathLibrary.VSize` (- (`.position_4_82183DE542908D596C8FAEB035EBD154` (break `/Game/Environment/Castle/AttackLocation` _array_element)) (`local.searchLocation`))))
        (if (< _returnvalue (`local.CurrentMin`))
          (set `local.CurrentMin` _returnvalue)
          (set `local.CurrentBestVector` (`.position_4_82183DE542908D596C8FAEB035EBD154` (break `/Game/Environment/Castle/AttackLocation` _array_element)))
          (set `local.CurrentBestIndex` _array_index))))
    (`KismetArrayLibrary.Array_Set` (`self.RangedLocations`) (`local.CurrentBestIndex`) (make `/Game/Environment/Castle/AttackLocation` false (`local.CurrentBestVector`)))
    (return (`local.CurrentBestVector`) (`local.CurrentBestIndex`))))

(fn `GetClosestWall`
  (params (Location :type "Vector Structure"))
  (returns (WallCollider :type "BoxComponent Object Reference"))
  (locals (BestCollider :type "BoxComponent Object Reference") (BestDistance :type "Float (double-precision)" :default 1000000000.0))
  (bind _keys (`BlueprintMapLibrary.Map_Keys` (`self.ColliderToStruct`)))
  (for _array_element _keys
    (bind _returnvalue (`KismetMathLibrary.VSize` (- (`SceneComponent.K2_GetComponentLocation` _array_element) (`local.Location`))))
    (if (< _returnvalue (`local.BestDistance`))
      (set `local.BestDistance` _returnvalue)
      (set `local.BestCollider` _array_element)))
  (return (`local.BestCollider`)))

(fn `PopulateMap`
  (params (WallScenes :type "Array of SceneComponent Object Reference (by ref)") (WallHealth :type "Float (double-precision)" :default 200.0))
  (locals (Wall :type "/Game/Environment/Castle/Wall Structure") (currentBox :type "BoxComponent Object Reference"))
  (bind _currentbox (`local.currentBox`))
  (for _array_element WallScenes
    (for _array_element_2 (`SceneComponent.GetChildrenComponents` _array_element false)
      (switch `name` (`|GetArrayItem` (`ActorComponent.ComponentTags` _array_element_2))
        (:`Default`
          (bind _asbox_collision (cast `BoxComponent` _array_element_2))
          (set `local.currentBox` _asbox_collision))
        (:`up`
          (bind _asstatic_mesh_component (cast `StaticMeshComponent` _array_element_2))
          (setmembers `/Game/Environment/Castle/Wall` :`StructRef` (`local.Wall`) :`TopWall` _asstatic_mesh_component))
        (:`mid`
          (bind _asstatic_mesh_component_2 (cast `StaticMeshComponent` _array_element_2))
          (setmembers `/Game/Environment/Castle/Wall` :`StructRef` (`local.Wall`) :`MidWall` _asstatic_mesh_component_2))
        (:`bot`
          (bind _asstatic_mesh_component_3 (cast `StaticMeshComponent` _array_element_2))
          (setmembers `/Game/Environment/Castle/Wall` :`StructRef` (`local.Wall`) :`BotWall` _asstatic_mesh_component_3))
        (:`u_dm`
          (bind _asdestructible_component (cast `DestructibleComponent` _array_element_2))
          (setmembers `/Game/Environment/Castle/Wall` :`StructRef` (`local.Wall`) :`DestructibleTop` _asdestructible_component))
        (:`b_dm`
          (bind _asdestructible_component_2 (cast `DestructibleComponent` _array_element_2))
          (setmembers `/Game/Environment/Castle/Wall` :`StructRef` (`local.Wall`) :`DestructibleBottom` _asdestructible_component_2))
        (:`m_dm`
          (bind _asdestructible_component_3 (cast `DestructibleComponent` _array_element_2))
          (setmembers `/Game/Environment/Castle/Wall` :`StructRef` (`local.Wall`) :`DestructibleMiddle` _asdestructible_component_3))))
    (bind _returnvalue (`AddComponent|NODE_AddWidgetComponent-0` :`self` self :`bManualAttachment` true))
    (`SceneComponent.K2_AttachToComponent` _returnvalue _currentbox "None" "KeepWorld" "KeepWorld" "KeepWorld" false)
    (`SceneComponent.K2_SetWorldLocation` _returnvalue (+ (`SceneComponent.K2_GetComponentLocation` _currentbox) (0.0 0.0 1000.0)) false false)
    (`SceneComponent.SetWorldScale3D` _returnvalue (1.0 20.0 6.0))
    (`WidgetComponent.SetManuallyRedraw` _returnvalue true)
    (bind _ashealth_bar (cast `/Game/UI/HealthBar` (`WidgetComponent.GetUserWidgetObject` _returnvalue)))
    (bind _structout (setmembers `/Game/Environment/Castle/Wall` :`StructRef` (`local.Wall`) :`Health` (`local.WallHealth`) :`HealthBarComponent` _returnvalue :`HealthBarWidget` _ashealth_bar))
    (`BlueprintMapLibrary.Map_Add` (`self.ColliderToStruct`) (`local.currentBox`) _structout)))

(fn `SetupVisibility`
  (bind _keys (`BlueprintMapLibrary.Map_Keys` (`self.ColliderToStruct`)))
  (for _array_element _keys
    (bind _value (`BlueprintMapLibrary.Map_Find` (`self.ColliderToStruct`) _array_element))
    (`SceneComponent.SetVisibility` (break `/Game/Environment/Castle/Wall` _value) false false)
    (`SceneComponent.SetVisibility` (`.DestructibleMiddle_8_804BC4774E57CFC6422A10BCFE3C892D` (break `/Game/Environment/Castle/Wall` _value)) false false)
    (`SceneComponent.SetVisibility` (`.DestructibleBottom_6_D50AC0344FA29EEEEEC606ABEC93D052` (break `/Game/Environment/Castle/Wall` _value)) false false)
    (`PrimitiveComponent.SetCollisionEnabled` (break `/Game/Environment/Castle/Wall` _value) "NoCollision")
    (`PrimitiveComponent.SetCollisionEnabled` (`.DestructibleMiddle_8_804BC4774E57CFC6422A10BCFE3C892D` (break `/Game/Environment/Castle/Wall` _value)) "NoCollision")
    (`PrimitiveComponent.SetCollisionEnabled` (`.DestructibleBottom_6_D50AC0344FA29EEEEEC606ABEC93D052` (break `/Game/Environment/Castle/Wall` _value)) "NoCollision")))

(fn `UserConstructionScript`)

(fn `WidgetsFaceCamera`
  (locals (CameraLocation :type "Vector Structure"))
  (set `local.CameraLocation` (`PlayerCameraManager.GetCameraLocation` (`GameplayStatics.GetPlayerCameraManager` 0)))
  (bind _values (`BlueprintMapLibrary.Map_Values` (`self.ColliderToStruct`)))
  (for _array_element _values
    (bind (_returnvalue_roll _returnvalue_pitch _returnvalue_yaw) (`KismetMathLibrary.BreakRotator` (`KismetMathLibrary.FindLookAtRotation` (`SceneComponent.K2_GetComponentLocation` (`.HealthBarComponent_26_665D88C949CD98398E6CC8A35D21A461` (break `/Game/Environment/Castle/Wall` _array_element))) (`local.CameraLocation`))))
    (`SceneComponent.K2_SetWorldRotation` (`.HealthBarComponent_26_665D88C949CD98398E6CC8A35D21A461` (break `/Game/Environment/Castle/Wall` _array_element)) (`KismetMathLibrary.MakeRotator` 0.0 0.0 _returnvalue_yaw) false false)))