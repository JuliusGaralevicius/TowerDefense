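; Player castle Blueprint for the tower defense mode, which registers itself with the game mode on spawn.
; Goblins overlapping its capsule are destroyed and counted, and the count is passed with total capacity to CallGoblinConsumed and printed on screen.
; A box trigger plays a timeline that lerps the gates 500 units upward when the playable character enters, and reverses it on exit.
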(event `self.ReceiveBeginPlay`
  (`parent.ReceiveBeginPlay`)
  (bind _astower_defense_game_mode (cast `/Game/Modes/TowerDefenseGameMode` (`GameplayStatics.GetGameMode`)))
  (`/Game/Modes/TowerDefenseGameMode.OnPlayerCastleSpawned` _astower_defense_game_mode self)
  (bind _output_get (set `self.GatesStart` (`SceneComponent.K2_GetComponentLocation` (`self.CastleGates`))))
  (set `self.GatesEnd` (+ _output_get (0.0 0.0 500.0))))

(event `self.Capsule.OnComponentBeginOverlap`
  (params (OverlappedComponent :type "PrimitiveComponent Object Reference") (OtherActor :type "Actor Object Reference") (OtherComp :type "PrimitiveComponent Object Reference") (OtherBodyIndex :type Integer) (bFromSweep :type Boolean) (SweepResult :type "HitResult Structure (by ref)"))
  (bind _goblinsconsumed (`self.goblinsConsumed`))
  (bind _asgoblin_base (cast `/Game/Characters/Goblins/GoblinBase/GoblinBase` OtherActor))
  (`self.K2_DestroyActor` _asgoblin_base)
  (bind _result (`/Engine/EditorBlueprintResources/StandardMacros.IncrementInt` _goblinsconsumed)
    (:`  `
      (`self.GoblinConsumed` (`self.totalGoblinCapacity`) _result)
      (`KismetSystemLibrary.PrintString` (`KismetStringLibrary.Conv_IntToString` _goblinsconsumed)))))

(event `self.Box.OnComponentBeginOverlap`
  (params (OverlappedComponent :type "PrimitiveComponent Object Reference") (OtherActor :type "Actor Object Reference") (OtherComp :type "PrimitiveComponent Object Reference") (OtherBodyIndex :type Integer) (bFromSweep :type Boolean) (SweepResult :type "HitResult Structure (by ref)"))
  (cast `/Game/Characters/PlayableCharacter` OtherActor)
  (bind (_direction _track) (`Timeline|Timeline_0` :!label _label)
    (:`Update`
      (`SceneComponent.K2_SetWorldLocation` (`self.CastleGates`) (`KismetMathLibrary.VLerp` (`self.GatesStart`) (`self.GatesEnd`) _track) false false))))

(event `self.Box.OnComponentEndOverlap`
  (params (OverlappedComponent :type "PrimitiveComponent Object Reference") (OtherActor :type "Actor Object Reference") (OtherComp :type "PrimitiveComponent Object Reference") (OtherBodyIndex :type Integer))
  (cast `/Game/Characters/PlayableCharacter` OtherActor)
  (goto _label :!via `Reverse`))

(fn `UserConstructionScript`
  (`parent.UserConstructionScript`))