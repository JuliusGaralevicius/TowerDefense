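; Item_BP is a world item pickup that goes into the inventory of whoever interacts with it.
; On Interact, it finds the interactor's InventoryComponent_BP and passes it a slot structure built from its item data and quantity.
; If the add succeeds, it calls ToggleInventory twice in succession, then destroys itself.
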(event `/Game/Interactable.Interact`
  (params (Interactor :type "Actor Object Reference"))
  (bind _returnvalue (`self.GetComponentByClass` Interactor "/Game/InventorySystem/InventoryComponent_BP.InventoryComponent_BP_C"))
  (if (`KismetSystemLibrary.IsValid` _returnvalue)
    (bind _success (`/Game/InventorySystem/InventoryComponent_BP.AddToInventory` _returnvalue (make `/Game/InventorySystem/SlotStructure` (`self.QuantityValue`) (`self.ItemStructure`))))
    (if _success
      (`/Game/InventorySystem/InventoryComponent_BP.ToggleInventory` _returnvalue)
      (`/Game/InventorySystem/InventoryComponent_BP.ToggleInventory` _returnvalue)
      (`self.K2_DestroyActor`))))

(fn `UserConstructionScript`)