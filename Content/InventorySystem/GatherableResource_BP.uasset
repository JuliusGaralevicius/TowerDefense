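; Gatherable resource actor that, after being interacted with for a set time, spawns a quantity of items and destroys itself.
; Interact records the interactor and enables Tick, which accumulates time until the processing threshold is reached.
; Items then spawn at randomly scattered offsets around the actor, and the empty Processed hook runs before destruction.
; When the last interactor ends overlap, progress resets and Tick is disabled.
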(event `/Game/Interactable.Interact`
  (params (Interactor :type "Actor Object Reference"))
  (set `self.isInteracting` true)
  (`self.SetActorTickEnabled` self true)
  (set `self.lastInteractor` Interactor))

(event `self.ReceiveTick`
  (params (DeltaSeconds :type "Float (single-precision)"))
  (bind (_returnvalue_x _returnvalue_y _returnvalue_z) (`KismetMathLibrary.BreakVector` (`self.K2_GetActorLocation`)))
  (if (`self.isInteracting`)
    (bind _output_get (set `self.timeInteracted` (+ DeltaSeconds (`self.timeInteracted`))))
    (if (>= _output_get (`self.TimeToProccess`))
      (for _ (range 1 (+ (`self.SpawnedItemQuantity`) 1))
        (`|SpawnActorFromClass` (`self.ItemToSpawn`) (`KismetMathLibrary.MakeTransform` (`KismetMathLibrary.MakeVector` (+ _returnvalue_x (`KismetMathLibrary.RandomFloatInRange` -100.0 200.0)) (+ _returnvalue_y (`KismetMathLibrary.RandomFloatInRange` -100.0 200.0)) (+ _returnvalue_z (`KismetMathLibrary.RandomFloatInRange` 10.0 30.0)))) "AdjustIfPossibleButAlwaysSpawn" "OverrideRootScale" null null))
      (`self.Processed`)
      (`self.K2_DestroyActor` self))))

(event `self.ReceiveActorEndOverlap`
  (params (OtherActor :type "Actor Object Reference"))
  (if (== OtherActor (`self.lastInteractor`))
    (set `self.isInteracting` false)
    (set `self.timeInteracted` 0.0)
    (`self.SetActorTickEnabled` self false)))

(fn `Processed`)

(fn `UserConstructionScript`)