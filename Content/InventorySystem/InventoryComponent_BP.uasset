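; Inventory actor component that holds a fixed number of item slots and toggles the player's inventory window.
; Adding an item tops up the first partial stack of the same class, recursively re-adding any overflow, or splits it into new max-size stacks.
; New stacks fill slots found by searching for a zero-quantity entry.
; Toggling adds or removes the widget on the custom controller's canvas and switches cursor and input mode.
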(event `self.ReceiveBeginPlay`
  (`self.PrepareInventory`))

(fn `AddToInventory`
  (params (ContentToAdd :type "/Game/InventorySystem/SlotStructure Structure"))
  (returns (Success :type Boolean))
  (if (`.Stackable_12_28DA4CE148203BBE6EC8F5A59ABD783E` (break `/Game/InventorySystem/ItemStructure` (`.Item_3_383DEDE1403944D5A1C3A8BA872460B0` (break `/Game/InventorySystem/SlotStructure` ContentToAdd))))
    (bind (_has_partial_stack _index_of_stack) (`self.HasPartialStackF` self (`local.ContentToAdd`)))
    (if _has_partial_stack
      (`self.AddToStack` self (`local.ContentToAdd`) _index_of_stack)
      (else
        (`self.CreateStack` self (`local.ContentToAdd`) :!label _label)))
    (else
      (goto _label)))
  (return true))

(fn `AddToStack`
  (params (Contents :type "/Game/InventorySystem/SlotStructure Structure") (Index :type Integer))
  (returns (Success :type Boolean))
  (locals (CurrentStackQuantity :type Integer) (ItemsLeft :type Integer))
  (bind _contents_quantity (break `/Game/InventorySystem/SlotStructure` (`local.Contents`)))
  (bind _contents (`local.Contents`))
  (bind (_contents_quantity_2 _contents_item) (break `/Game/InventorySystem/SlotStructure` (`local.Contents`)))
  (bind (_contents_quantity_3 _contents_item_2) (break `/Game/InventorySystem/SlotStructure` (`local.Contents`)))
  (bind _output (`|GetArrayItem` (`self.Items`) Index))
  (bind (_output_quantity _output_item) (break `/Game/InventorySystem/SlotStructure` (`|GetArrayItem` (`self.Items`) (`local.Index`))))
  (bind _returnvalue (+ Contents_Quantity_5_4BD0F0BF4777241859C21B8FD29503C6 (break `/Game/InventorySystem/SlotStructure` _output)))
  (set `local.CurrentStackQuantity` _returnvalue)
  (if (<= _returnvalue (`.MaxStackSize_23_F5346940432E704CC751368A21BC907C` (break `/Game/InventorySystem/ItemStructure` (`.Item_3_383DEDE1403944D5A1C3A8BA872460B0` (break `/Game/InventorySystem/SlotStructure` _output)))))
    (`KismetArrayLibrary.Array_Set` (`self.Items`) (`local.Index`) (make `/Game/InventorySystem/SlotStructure` (+ _output_quantity _contents_quantity) _output_item))
    (else
      (`KismetArrayLibrary.Array_Set` (`self.Items`) (`local.Index`) (make `/Game/InventorySystem/SlotStructure` (`.MaxStackSize_23_F5346940432E704CC751368A21BC907C` (break `/Game/InventorySystem/ItemStructure` (`.Item_3_383DEDE1403944D5A1C3A8BA872460B0` (break `/Game/InventorySystem/SlotStructure` _contents)))) _contents_item_2))
      (`self.AddToInventory` (make `/Game/InventorySystem/SlotStructure` (- (`local.CurrentStackQuantity`) (`.MaxStackSize_23_F5346940432E704CC751368A21BC907C` (break `/Game/InventorySystem/ItemStructure` (`.Item_3_383DEDE1403944D5A1C3A8BA872460B0` (break `/Game/InventorySystem/SlotStructure` _contents))))) _contents_item))))
  (return true))

(fn `CreateStack`
  (params (ContentToAdd :type "/Game/InventorySystem/SlotStructure Structure"))
  (locals (currentItemCount :type Integer))
  (bind (_contenttoadd_quantity _contenttoadd_item) (break `/Game/InventorySystem/SlotStructure` (`local.ContentToAdd`)))
  (bind (_contenttoadd_quantity_2 _contenttoadd_item_2) (break `/Game/InventorySystem/SlotStructure` (`local.ContentToAdd`)))
  (bind _items (`self.Items`))
  (bind _output_get (set `local.currentItemCount` ContentToAdd_Quantity_5_4BD0F0BF4777241859C21B8FD29503C6))
  (while (>= _output_get (`.MaxStackSize_23_F5346940432E704CC751368A21BC907C` (break `/Game/InventorySystem/ItemStructure` (`.Item_3_383DEDE1403944D5A1C3A8BA872460B0` (break `/Game/InventorySystem/SlotStructure` ContentToAdd)))))
    (set `local.currentItemCount` (- (`local.currentItemCount`) (`.MaxStackSize_23_F5346940432E704CC751368A21BC907C` (break `/Game/InventorySystem/ItemStructure` (`.Item_3_383DEDE1403944D5A1C3A8BA872460B0` (break `/Game/InventorySystem/SlotStructure` ContentToAdd))))))
    (`KismetArrayLibrary.Array_Set` _items (`KismetArrayLibrary.Array_Find` _items (make `/Game/InventorySystem/SlotStructure` 0)) (make `/Game/InventorySystem/SlotStructure` (`.MaxStackSize_23_F5346940432E704CC751368A21BC907C` (break `/Game/InventorySystem/ItemStructure` (`.Item_3_383DEDE1403944D5A1C3A8BA872460B0` (break `/Game/InventorySystem/SlotStructure` ContentToAdd)))) _contenttoadd_item)))
  (if (not (== (`local.currentItemCount`) 0))
    (`KismetArrayLibrary.Array_Set` (`self.Items`) (`KismetArrayLibrary.Array_Find` (`self.Items`) (make `/Game/InventorySystem/SlotStructure` 0)) (make `/Game/InventorySystem/SlotStructure` (`local.currentItemCount`) _contenttoadd_item_2)))
  (return))

(fn `HasPartialStackF`
  (params (InputItems :type "/Game/InventorySystem/SlotStructure Structure"))
  (returns (`Has Partial Stack` :type Boolean) (`Index of stack` :type Integer))
  (locals (StackFound :type Boolean) (Index :type Integer))
  (bind _inputitems (`local.InputItems`))
  (for (_array_element _array_index) (`self.Items`)
    (if (and (< (break `/Game/InventorySystem/SlotStructure` _array_element) (`.MaxStackSize_23_F5346940432E704CC751368A21BC907C` (break `/Game/InventorySystem/ItemStructure` (`.Item_3_383DEDE1403944D5A1C3A8BA872460B0` (break `/Game/InventorySystem/SlotStructure` _inputitems))))) (== (`.Class_20_47AA2D5B41D25945229AA99D21E5F612` (break `/Game/InventorySystem/ItemStructure` (`.Item_3_383DEDE1403944D5A1C3A8BA872460B0` (break `/Game/InventorySystem/SlotStructure` _array_element)))) (`.Class_20_47AA2D5B41D25945229AA99D21E5F612` (break `/Game/InventorySystem/ItemStructure` (`.Item_3_383DEDE1403944D5A1C3A8BA872460B0` (break `/Game/InventorySystem/SlotStructure` _inputitems))))))
      (set `local.StackFound` true)
      (set `local.Index` _array_index)
      (break)))
  (return (`local.StackFound`) (`local.Index`)))

(fn `PrepareInventory`
  (`KismetArrayLibrary.Array_Resize` (`self.Items`) (`self.NumberOfSlots`)))

(fn `ToggleInventory`
  (bind _returnvalue (`GameplayStatics.GetPlayerController` 0))
  (bind _inventorywindow (`self.InventoryWindow`))
  (`/Engine/EditorBlueprintResources/StandardMacros.IsValid` _inventorywindow
    (:`Is Valid`
      (`Widget.RemoveFromParent` _inventorywindow)
      (set `self.InventoryWindow` null)
      (`WidgetBlueprintLibrary.SetInputMode_GameOnly` (`GameplayStatics.GetPlayerController` 0))
      (set `PlayerController.bShowMouseCursor` false (`GameplayStatics.GetPlayerController` 0)))
    (:`Is Not Valid`
      (bind _returnvalue_2 (`|CreateWidget` "/Game/InventorySystem/InventoryUI/InventoryWidget.InventoryWidget_C" null self))
      (bind _output_get (set `self.InventoryWindow` _returnvalue_2))
      (bind _ascustom_player_controller (cast `/Game/Assets/Blueprints/CustomPlayerController` (`GameplayStatics.GetPlayerController` 0)))
      (bind _canvaspanel (`/Game/Assets/Blueprints/CustomPlayerController.GetPlayerCanvas` _ascustom_player_controller))
      (bind _returnvalue_3 (`CanvasPanel.AddChildToCanvas` _canvaspanel _output_get))
      (`CanvasPanelSlot.SetAutoSize` _returnvalue_3 true)
      (`CanvasPanelSlot.SetAnchors` _returnvalue_3 (make `Anchors` (0.65 0.2) (0.65 0.2)))
      (set `PlayerController.bShowMouseCursor` true _returnvalue)
      (`WidgetBlueprintLibrary.SetInputMode_GameAndUIEx` _returnvalue null "LockAlways"))))