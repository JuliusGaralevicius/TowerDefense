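; Gatherable resource actor that turns into item drops when interacted with.
; Interact spawns the configured quantity of the item class at random offsets around and slightly above the actor, adjusting for collision but always spawning.
; It then calls Processed, an empty hook here, and destroys itself.
; RequestInteractTIme always reports success and returns ProcessTime as the interaction duration.
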(event `/Game/Interfaces/Interactable.Interact`
  (params (Interactor :type "Actor Object Reference"))
  (bind (_returnvalue_x _returnvalue_y _returnvalue_z) (`KismetMathLibrary.BreakVector` (`self.K2_GetActorLocation`)))
  (for _ (range 1 (+ (`self.SpawnedItemQuantity`) 1))
    (`|SpawnActorFromClass` (`self.ItemToSpawn`) (`KismetMathLibrary.MakeTransform` (`KismetMathLibrary.MakeVector` (+ _returnvalue_x (`KismetMathLibrary.RandomFloatInRange` -100.0 200.0)) (+ _returnvalue_y (`KismetMathLibrary.RandomFloatInRange` -100.0 200.0)) (+ _returnvalue_z (`KismetMathLibrary.RandomFloatInRange` 10.0 30.0)))) "AdjustIfPossibleButAlwaysSpawn" "OverrideRootScale" null null))
  (`self.Processed`)
  (`self.K2_DestroyActor` self))

(fn `Processed`)

(fn `RequestInteractTIme`
  (returns (success :type Boolean) (Time :type "Float (double-precision)"))
  (return true (`self.ProcessTime`)))

(fn `UserConstructionScript`)