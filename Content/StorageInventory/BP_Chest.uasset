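; BP_Chest is an interactable storage chest that opens its storage inventory for a player.
; On Interact it stores the interacting PlayableCharacter and tells it to display the chest's Storage.
; When a playable character leaves the ExitInventoryCollider, that character hides the storage display.
; The interaction duration is supplied by RequestInteractTIme from the OpenTime variable.
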(event `/Game/Interfaces/Interactable.Interact`
  (params (Interactor :type "Actor Object Reference"))
  (bind _asplayable_character (cast `/Game/Characters/PlayableCharacter` Interactor))
  (bind _output_get (set `self.PlayerInteractor` _asplayable_character))
  (`/Game/Characters/PlayableCharacter.Display Storage Inventory` _asplayable_character (`self.Storage`) true)
  (`/Game/Characters/PlayableCharacter.Display Storage Inventory` _output_get (`self.Storage`) true))

(event `self.ExitInventoryCollider.OnComponentEndOverlap`
  (params (OverlappedComponent :type "PrimitiveComponent Object Reference") (OtherActor :type "Actor Object Reference") (OtherComp :type "PrimitiveComponent Object Reference") (OtherBodyIndex :type Integer))
  (bind _asplayable_character (cast `/Game/Characters/PlayableCharacter` OtherActor))
  (`/Game/Characters/PlayableCharacter.Display Storage Inventory` _asplayable_character (`self.Storage`) false))

(fn `RequestInteractTIme`
  (returns (success :type Boolean) (Time :type "Float (double-precision)"))
  (return true (`self.OpenTime`)))

(fn `UserConstructionScript`)