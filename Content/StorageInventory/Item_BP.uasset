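; Item_BP is an interactable world pickup that adds its item to the interacting player's inventory.
; On Interact it casts the interactor to PlayableCharacter and, for non-weapon items, passes its ItemStructure to InventoryComponentUpdated.AddItem, destroying itself only if the add succeeds.
; Weapon-flagged items do nothing on interaction here.
; It also reports its PickupTime as the interaction duration through RequestInteractTIme.
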(event `/Game/Interfaces/Interactable.Interact`
  (params (Interactor :type "Actor Object Reference"))
  (bind _asplayable_character (cast `/Game/Characters/PlayableCharacter` Interactor))
  (if (not (`self.IsWeapon`))
    (bind _success (`/Game/CharacterInventory/Inventory.AddItem` (`/Game/Characters/PlayableCharacter.InventoryComponentUpdated` _asplayable_character) (`self.ItemStructure`)))
    (if _success
      (`self.K2_DestroyActor`))))

(fn `RequestInteractTIme`
  (returns (success :type Boolean) (Time :type "Float (double-precision)"))
  (return true (`self.PickupTime`)))

(fn `UserConstructionScript`)