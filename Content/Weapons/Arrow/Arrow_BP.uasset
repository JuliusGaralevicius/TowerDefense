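; Arrow projectile actor that deals damage to what it hits.
; The construction script sets the projectile movement's velocity from InitialVelocity.
; On capsule overlap it ignores its Instigator, casts the other actor to DamageReceiver, passes Damage to OnReceiveDamage and destroys itself.
; Overlaps with actors that fail the cast leave the arrow alive.
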(event `self.Capsule.OnComponentBeginOverlap`
  (params (OverlappedComponent :type "PrimitiveComponent Object Reference") (OtherActor :type "Actor Object Reference") (OtherComp :type "PrimitiveComponent Object Reference") (OtherBodyIndex :type Integer) (bFromSweep :type Boolean) (SweepResult :type "HitResult Structure (by ref)"))
  (if (!= OtherActor (`self.Instigator`))
    (bind _asdamage_receiver (cast `/Game/Interfaces/DamageReceiver` OtherActor))
    (`/Game/Interfaces/DamageReceiver.OnReceiveDamage` _asdamage_receiver (`self.Damage`))
    (`self.K2_DestroyActor`)))

(fn `UserConstructionScript`
  (set `MovementComponent.Velocity` (`self.Initial Velocity`) (`self.ProjectileMovement`)))